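; BP_PlayerPawn is a player pawn Blueprint that manages its on-screen crosshair and health indicator widgets.
; On BeginPlay, only when locally controlled, it creates both widgets, adds them to the viewport and stores references.
; On Destroyed, it removes whichever widgets exist from their parent.
; The HealthComponent's OnHealthChanged handler and the construction script are empty.
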(event `self.ReceiveBeginPlay`
  (if (`self.IsLocallyControlled`)
    (`|ExecutionSequence`
      (:`then_0`
        (bind _returnvalue (`|CreateWidget` "/Game/UI/WBP_Crosshair.WBP_Crosshair_C"))
        (`UserWidget.AddToViewport` _returnvalue 0)
        (set `self.Crosshair` _returnvalue))
      (:`then_1`
        (bind _returnvalue_2 (`|CreateWidget` "/Game/UI/WBP_HealthIndicator.WBP_HealthIndicator_C"))
        (`UserWidget.AddToViewport` _returnvalue_2 0)
        (set `self.HealthIndicator` _returnvalue_2)))))

(event `self.ReceiveDestroyed`
  (bind _crosshair (`self.Crosshair`))
  (bind _healthindicator (`self.HealthIndicator`))
  (if (!= _crosshair null)
    (`Widget.RemoveFromParent` _crosshair))
  (if (!= _healthindicator null)
    (`Widget.RemoveFromParent` _healthindicator)))

(event `self.HealthComponent.OnHealthChanged`
  (params (HealthComponent :type "SHealthComponent Object Reference") (CurrentHealth :type "Float (single-precision)") (HealthDelta :type "Float (single-precision)") (DamageType :type "DamageType Object Reference") (InstigatedBy :type "Controller Object Reference") (DamageCauser :type "Actor Object Reference")))

(fn `UserConstructionScript`)